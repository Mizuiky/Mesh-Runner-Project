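; AI controller that drives a BP_Runner pawn by simulating alternating left and right power inputs.
; On possess it caches the runner, and on BeginPlay it starts a randomly delayed timer.
; SimulateInput flip-flops between the runner's left and right power calls, rescheduling after each with a new random delay between the min and max input delays.
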(event `self.ReceiveBeginPlay`
  (`self.SimulatInputWithDelay`))

(event `self.ReceivePossess`
  (params (PossessedPawn :type "Pawn Object Reference"))
  (bind _asbp_runner (cast `/Game/Blueprints/BP_Runner` PossessedPawn))
  (set `self.AIRunner` _asbp_runner))

(event `SimulateInput`
  (`/Engine/EditorBlueprintResources/StandardMacros.FlipFlop`
    (:`A`
      (`/Game/Blueprints/BP_Runner.SimulatePowerLeft` (`self.AIRunner`))
      (`self.SimulatInputWithDelay`))
    (:`B`
      (`/Game/Blueprints/BP_Runner.SimulatePowerRight` (`self.AIRunner`))
      (`self.SimulatInputWithDelay`))))

(fn `SimulatInputWithDelay`
  (`KismetSystemLibrary.K2_SetTimerDelegate` (`|CreateDelegate` :!event `SimulateInput`) (`KismetMathLibrary.RandomFloatInRange` (`self.MinInputDelay`) (`self.MaxInputDelay`))))

(fn `UserConstructionScript`)
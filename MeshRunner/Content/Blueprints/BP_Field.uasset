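; BP_Field is a 2D stage actor that builds a modular playfield from repeated field sprites, with top and bottom boxes and goals.
; Its construction script adds StageParts Paper sprites along X, spaced by StageLength.
; It then stretches and centers both boxes over the full run and offsets both goals to the last part, adding to their existing X position.
; All logic runs at construction, leaving the event graph empty.
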(fn `SetGoalLocation`
  (params (Goal :type "ChildActorComponent Object Reference"))
  (bind (_relativelocation_x _relativelocation_y _relativelocation_z) (`KismetMathLibrary.BreakVector` (`SceneComponent.RelativeLocation` Goal)))
  (`SceneComponent.K2_SetRelativeLocation` Goal (`KismetMathLibrary.MakeVector` (+ (* (- (`self.Stage Parts`) 1) (`self.Stage Length`)) _relativelocation_x) _relativelocation_y _relativelocation_z) false false))

(fn `UpdateBoxExtents`
  (params (Box :type "BoxComponent Object Reference"))
  (bind (_boxextent_x _boxextent_y _boxextent_z) (`KismetMathLibrary.BreakVector` (`BoxComponent.BoxExtent` Box)))
  (`BoxComponent.SetBoxExtent` Box (`KismetMathLibrary.MakeVector` (`KismetMathLibrary.Conv_IntToDouble` (* (/ (`self.Stage Length`) 2) (`self.Stage Parts`))) _boxextent_y _boxextent_z) true))

(fn `UpdateBoxLocation`
  (params (Box :type "SceneComponent Object Reference"))
  (bind (_relativelocation_x _relativelocation_y _relativelocation_z) (`KismetMathLibrary.BreakVector` (`SceneComponent.RelativeLocation` Box)))
  (`SceneComponent.K2_SetRelativeLocation` Box (`KismetMathLibrary.MakeVector` (`KismetMathLibrary.Conv_IntToDouble` (- (/ (* (`self.Stage Length`) (`self.Stage Parts`)) 2) (/ (`self.Stage Length`) 2))) _relativelocation_y _relativelocation_z) false false))

(fn `UserConstructionScript`
  (for _index (range (`self.Stage Parts`))
    (bind _returnvalue (`AddComponent|NODE_AddPaperSpriteComponent-0` :`RelativeTransform` (`KismetMathLibrary.MakeTransform` (`KismetMathLibrary.MakeVector` (`KismetMathLibrary.Conv_IntToDouble` (* _index (`self.Stage Length`)))))))
    (`PaperSpriteComponent.SetSprite` _returnvalue "/Game/PaperAssets/Background/T_Field_Sprite.T_Field_Sprite"))
  (`self.UpdateBoxExtents` (`self.BoxTop`))
  (`self.UpdateBoxExtents` (`self.BoxBottom`))
  (`self.UpdateBoxLocation` (`self.BoxTop`))
  (`self.UpdateBoxLocation` (`self.BoxBottom`))
  (`self.SetGoalLocation` (`self.GoalTop`))
  (`self.SetGoalLocation` (`self.Goal Bottom`)))